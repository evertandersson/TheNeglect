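; BP_Door is an interactable door whose behavior follows a state: open, close, locked, partially open, keyhole peek, missing handle or cutscene trigger.
; The InteractableComponent's dispatcher runs the state switch, playing sounds and setting a yaw target that Tick interpolates toward.
; Key and handle states consume player inventory items, with overlap unlocking the referenced Dooropen.
; Keyhole viewing temporarily moves the player camera and can partially open BP_DoorBathroom, found by name.
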(event `self.ReceiveBeginPlay`
  (bind _returnvalue (`GameplayStatics.GetActorOfClass` "/Game/ThirdPerson/Blueprints/BP_FirstPerson.BP_FirstPerson_C"))
  (set `self.PlayerRef` _returnvalue)
  (add `/Game/Alexander/InteractableComponent.OnInteractDispatcher` (`self.InteractableComponent`) (delegate `BeginInteractLogic`))
  (switch `/Game/Alexander/E_DoorInteractState` (`self.DoorInteractState`)
    (:`NewEnumerator5`
      (`SceneComponent.SetVisibility` (`self.SM_door_v3_LP_handle_1_low`) false false))))

(event `BeginInteractLogic`
  (bind _dooropen (`self.Dooropen`))
  (bind _firstpersoncamera (`GP3_Team2Character.FirstPersonCamera` (`self.PlayerRef`)))
  (bind _inventory (`/Game/ThirdPerson/Blueprints/BP_FirstPerson.Inventory` (`self.PlayerRef`)))
  (`KismetSystemLibrary.PrintString` "Door interact logic activated")
  (switch `/Game/Alexander/E_DoorInteractState` (`self.DoorInteractState`)
    (:`NewEnumerator0`
      (`KismetSystemLibrary.PrintString` "Door is opened")
      (`GameplayStatics.PlaySound2D` "/Game/Kamil/SoundDesign/SFX/door/SC_openDoor.SC_openDoor" 1.0 1.0 0.0 null null)
      (set `self.IsRotating` true)
      (set `self.RotationTarget` 90.0)
      (set `self.DoorInteractState` "NewEnumerator1"))
    (:`NewEnumerator1`
      (`KismetSystemLibrary.PrintString` "Door is closed")
      (if (`self.bPlayDoorCloseSound`)
        (`GameplayStatics.SpawnSound2D` "/Game/Kamil/SoundDesign/SFX/door/doorclose.doorclose" 1.0 1.0 0.0 null)
        (set `self.bPlayDoorCloseSound` false))
      (set `self.IsRotating` true)
      (set `self.RotationTarget` 0.0)
      (set `self.DoorInteractState` "NewEnumerator0")
      (set `self.bIsClosing` true))
    (:`NewEnumerator2`
      (`KismetSystemLibrary.PrintString` "Door locked")
      (`GameplayStatics.PlaySound2D` "/Game/Kamil/SoundDesign/SFX/door/locked2_Cue.locked2_Cue" 1.0 1.0 0.0 null null)
      (if (`KismetSystemLibrary.IsValid` _dooropen)
        (if (`self.bhadBeenShown`)
          _
          (elif (`self.bDisplayLockText`)
            (`self.LockedDoorText` _dooropen)
            (`KismetSystemLibrary.PrintString` "asdasd")))))
    (:`NewEnumerator3`
      (`KismetSystemLibrary.PrintString` "partially open")
      (`GameplayStatics.PlaySound2D` "/Game/Kamil/SoundDesign/SFX/door/SC_partiallyOpen.SC_partiallyOpen" 1.0 1.0 0.0 null null)
      (set `self.IsRotating` true)
      (set `self.RotationTarget` 25.0)
      (set `self.DoorInteractState` "NewEnumerator0")
      (`KismetSystemLibrary.PrintString` "Hello"))
    (:`NewEnumerator4`
      (`KismetSystemLibrary.PrintString` "Lookthroughkeyhole")
      (bind _returnvalue (`GameplayStatics.GetActorOfClass` "/Game/Alexander/BP_InteractManager.BP_InteractManager_C"))
      (set `self.InteractManager` _returnvalue)
      (set `self.CameraTransform` (`SceneComponent.K2_GetComponentToWorld` _firstpersoncamera))
      (`SceneComponent.K2_SetWorldLocation` _firstpersoncamera (+ (100.0 10.0 77.5) (`self.K2_GetActorLocation`)) false false)
      (`SceneComponent.K2_SetWorldRotation` _firstpersoncamera (struct :`Yaw` -90.0) false false)
      (`self.DisableInput` (`self.PlayerRef`) (`GameplayStatics.GetPlayerController` 0))
      (`UserWidget.AddToViewport` (`/Game/Alexander/BP_InteractManager.KeyholeUI` (`self.InteractManager`)) 0)
      (`KismetSystemLibrary.Delay` (`self.KeyholeInteractDuration`))
      (`SceneComponent.K2_SetWorldTransform` (`GP3_Team2Character.FirstPersonCamera` (`self.PlayerRef`)) (`self.CameraTransform`) false false)
      (`self.EnableInput` (`self.PlayerRef`) (`GameplayStatics.GetPlayerController` 0))
      (`Widget.RemoveFromParent` (`/Game/Alexander/BP_InteractManager.KeyholeUI` (`self.InteractManager`)))
      (if (`self.IsLookThroughKeyholeLoop1`)
        (`self.LookThroughKeyHoleLoop1`)))
    (:`NewEnumerator5`
      (`KismetSystemLibrary.PrintString` "NoHandleLogic")
      (for _array_element _inventory
        (if (`KismetTextLibrary.EqualEqual_TextText` (`.Name_2_A3E831DF4990971A51349A8F831EA43C` (break `/Game/ThirdPerson/Blueprints/PickUpItemData` _array_element)) (`|FormatText` "Handle"))
          (`KismetArrayLibrary.Array_RemoveItem` _inventory _array_element)
          (`SceneComponent.SetVisibility` (`self.SM_door_v3_LP_handle_1_low`) true false)
          (set `self.DoorInteractState` "NewEnumerator0"))))
    (:`NewEnumerator6`
      (`KismetSystemLibrary.PrintString` "Start Seq")
      (set `self.bStartCutScene` true)
      (set `/Game/Alexander/InteractableComponent.IsInteractable` false (`self.InteractableComponent`)))))

(event `Unlock Door2`
  (set `self.DoorInteractState` "NewEnumerator0"))

(event `Unlock Door`
  (`GameplayStatics.PlaySound2D` "/Game/Kamil/SoundDesign/SFX/door/doorclose.doorclose" 1.0 1.0 0.0 null null)
  (set `self.DoorInteractState` "NewEnumerator0")
  (`KismetSystemLibrary.PrintString` "Door unlocked"))

(event `self.Box.OnComponentBeginOverlap`
  (params (OverlappedComponent :type "PrimitiveComponent Object Reference") (OtherActor :type "Actor Object Reference") (OtherComp :type "PrimitiveComponent Object Reference") (OtherBodyIndex :type Integer) (bFromSweep :type Boolean) (SweepResult :type "HitResult Structure (by ref)"))
  (bind _inventory (`/Game/ThirdPerson/Blueprints/BP_FirstPerson.Inventory` (`self.PlayerRef`)))
  (if (`KismetSystemLibrary.IsValid` (`self.Dooropen`))
    (bind _asbp_first_person (cast `/Game/ThirdPerson/Blueprints/BP_FirstPerson` OtherActor))
    (message `/Game/Kamil/Blueprints/InteractionArea/BPI_Interaction.InterfaceToggleFocus` (`self.Door`) true)
    (bind _has_key (`/Game/ThirdPerson/Blueprints/BP_FirstPerson.Has Key` _asbp_first_person))
    (if _has_key
      (if _has_key
        (`self.Unlock Door2` (`self.Dooropen`))
        (for _array_element _inventory
          (if (`KismetTextLibrary.EqualEqual_TextText` (`.Name_2_A3E831DF4990971A51349A8F831EA43C` (break `/Game/ThirdPerson/Blueprints/PickUpItemData` _array_element)) (`|FormatText` "Key"))
            (`KismetArrayLibrary.Array_RemoveItem` _inventory _array_element)))))))

(event `LockedDoorText`
  (set `self.bhadBeenShown` true)
  (bind _returnvalue (`|CreateWidget` "/Game/UI/WBP_LockedDoor.WBP_LockedDoor_C"))
  (bind _output_get (set `self.LoockedDoor` _returnvalue))
  (`UserWidget.AddToViewport` _output_get 0)
  (`KismetSystemLibrary.Delay` 4.0)
  (`Widget.RemoveFromParent` (`self.LoockedDoor`)))

(event `ParticallyOpenDoor`
  (set `self.DoorInteractState` "NewEnumerator3")
  (`self.BeginInteractLogic`))

(event `self.ReceiveTick`
  (params (DeltaSeconds :type "Float (single-precision)"))
  (if (`self.IsRotating`)
    (`self.HandleRotation` (`self.RotationTarget`))))

(event `HandleRotation`
  (params (SetRotation :type "Float (double-precision)"))
  (`SceneComponent.K2_SetRelativeRotation` (`self.Door`) (`KismetMathLibrary.MakeRotator` 0.0 0.0 (`KismetMathLibrary.FInterpTo` (.yaw (`SceneComponent.RelativeRotation` (`self.Door`))) SetRotation (`GameplayStatics.GetWorldDeltaSeconds`) (`self.Interp Speed`))) false false)
  (if (`self.bIsClosing`)
    (if (== (`SceneComponent.RelativeRotation` (`self.Door`)) (struct) :`ErrorTolerance` 0.5)
      (set `self.bPlayDoorCloseSound` true)
      (if (== (`SceneComponent.RelativeRotation` (`self.Door`)) (struct)) :!label _label
        (set `self.IsRotating` false)))
    (else
      (goto _label))))

(fn `LookThroughKeyHoleLoop1`
  (bind _outactors (`GameplayStatics.GetAllActorsOfClass` "BP_Door_C"))
  (for _array_element _outactors
    (if (`KismetStringLibrary.EqualEqual_StrStr` (`KismetSystemLibrary.GetDisplayName` _array_element) "BP_DoorBathroom")
      (set `self.BathroomDoor` _array_element)
      (set `/Game/Alexander/BP_Door.DoorInteractState` "NewEnumerator3" (`self.BathroomDoor`))
      (`self.BeginInteractLogic` (`self.BathroomDoor`)))))

(fn `UserConstructionScript`)
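; BP_Handle is an interactable door handle that highlights on focus and starts an interaction on the first-person player.
; On BeginPlay it caches BP_FirstPerson and binds its InteractableComponent's interact dispatcher to logic that calls InteractStart on the player.
; Focus changes toggle custom depth rendering on the handle mesh.
; GetMesh returns the item's name, mesh and icon.
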(event `self.ReceiveBeginPlay`
  (bind _returnvalue (`GameplayStatics.GetActorOfClass` "/Game/ThirdPerson/Blueprints/BP_FirstPerson.BP_FirstPerson_C"))
  (set `self.PlayerRef` _returnvalue)
  (add `/Game/Alexander/InteractableComponent.OnInteractDispatcher` (`self.InteractableComponent`) (delegate `BeginInteractLogic`)))

(event `BeginInteractLogic`
  (`KismetSystemLibrary.PrintString` "Handle interact logic activated")
  (`/Game/ThirdPerson/Blueprints/BP_FirstPerson.InteractStart` (`self.PlayerRef`)))

(event `/Game/Kamil/Blueprints/InteractionArea/BPI_Interaction.InterfaceToggleFocus`
  (params (Focus :type Boolean))
  (`PrimitiveComponent.SetRenderCustomDepth` (`self.SM_doorhandle_Lowpoly`) Focus))

(fn `GetMesh`
  (returns (Name :type Text) (`Static Mesh` :type "StaticMesh Object Reference") (`Item Icon` :type "Texture2D Object Reference"))
  (return "Handle" (`StaticMeshComponent.StaticMesh` (`self.SM_doorhandle_Lowpoly`)) (`self.ImageIcon`)))

(fn `UserConstructionScript`)
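; BP_Painting is a four-piece painting puzzle that partially opens a door once completed.
; On actor overlap it marks pieces the player holds as added, reveals their meshes and hides the item holder's puzzle-piece icon.
; When every entry in its piece-state array is added, it triggers the door once.
; An interface focus event toggles custom depth rendering on the painting for highlighting.
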(event `self.ReceiveBeginPlay`
  (for _index (range 4)
    (`KismetArrayLibrary.Array_Add` (`self.Painting Pieces`) (make `/Game/ThirdPerson/Blueprints/PuzzlePieceData` _index))))

(event `self.ReceiveActorBeginOverlap`
  (params (OtherActor :type "Actor Object Reference"))
  (bind _allpiecesareadded (`self.AllPiecesAreAdded`))
  (bind _returnvalue (`GameplayStatics.GetActorOfClass` "/Game/ThirdPerson/Blueprints/BP_FirstPerson.BP_FirstPerson_C"))
  (bind _bpitemholder (`/Game/ThirdPerson/Blueprints/BP_FirstPerson.GetItemHolder` _returnvalue))
  (set `self.WB_ItemHolder` _bpitemholder)
  (set `self.AllPiecesAreAdded` true)
  (for _array_element (`self.Painting Pieces`)
    (if (`.PlayerHasPiece_5_7E283E834A3D8EEF17AB7EABF20ECE86` (break `/Game/ThirdPerson/Blueprints/PuzzlePieceData` _array_element))
      (`self.SetPuzzlePiece` (break `/Game/ThirdPerson/Blueprints/PuzzlePieceData` _array_element) false true)
      (if (== (break `/Game/ThirdPerson/Blueprints/PuzzlePieceData` _array_element) 0)
        (`SceneComponent.SetHiddenInGame` (`self.Piece1`) false false)
        (elif (== (break `/Game/ThirdPerson/Blueprints/PuzzlePieceData` _array_element) 1)
          (`SceneComponent.SetHiddenInGame` (`self.Piece2`) false false)
          (elif (== (break `/Game/ThirdPerson/Blueprints/PuzzlePieceData` _array_element) 2)
            (`SceneComponent.SetHiddenInGame` (`self.Piece3`) false false)
            (elif (== (break `/Game/ThirdPerson/Blueprints/PuzzlePieceData` _array_element) 3)
              (`SceneComponent.SetHiddenInGame` (`self.Piece4`) false false)))))))
  (`/Game/Evert/WB_ItemHolder.HidePuzzlePieceIcon` (`self.WB_ItemHolder`))
  ;[1 1 1] Check if all pieces are collected
  (if (not (`self.IsTriggered`))
    (for _array_element_2 (`self.Painting Pieces`)
      (if _allpiecesareadded
        (if (`.PieceIsAdded_7_9667DD67491706680B720BB076946350` (break `/Game/ThirdPerson/Blueprints/PuzzlePieceData` _array_element_2))
          (set `self.AllPiecesAreAdded` true)
          (else
            (set `self.AllPiecesAreAdded` false :!label _label)))
        (else
          (goto _label))))
    (if _allpiecesareadded
      (`/Game/Alexander/BP_Door.ParticallyOpenDoor` (`self.Door`))
      (`KismetSystemLibrary.PrintString` "All pieces are collected")
      (set `self.IsTriggered` true))))

(event `/Game/Kamil/Blueprints/InteractionArea/BPI_Interaction.InterfaceToggleFocus`
  (params (Focus :type Boolean))
  (`PrimitiveComponent.SetRenderCustomDepth` (`self.Painting`) Focus))

(fn `SetPuzzlePiece`
  (params (Index :type Integer) (`Player has piece` :type Boolean) (`Piece Is Added` :type Boolean))
  (`KismetArrayLibrary.Array_Set` (`self.Painting Pieces`) Index (make `/Game/ThirdPerson/Blueprints/PuzzlePieceData` Index `Player has piece` `Piece Is Added`)))

(fn `UserConstructionScript`
  (set `self.IsTriggered` false))
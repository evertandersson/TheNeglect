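; BP_PuzzlePiece is an interactable puzzle piece that the player collects for a painting puzzle.
; BeginPlay applies the configured mesh and material, caches BP_FirstPerson and binds the interact dispatcher to call the player's InteractStart.
; Focus toggles custom depth on the mesh.
; GetPuzzlePiece reports the index as held but unplaced, while GetMesh returns item name, mesh and icon and, as a side effect, registers that state on the Painting.
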(event `/Game/Kamil/Blueprints/InteractionArea/BPI_Interaction.InterfaceToggleFocus`
  (params (Focus :type Boolean))
  (`PrimitiveComponent.SetRenderCustomDepth` (`self.PuzzlePiece`) Focus))

(event `self.ReceiveBeginPlay`
  (`StaticMeshComponent.SetStaticMesh` (`self.PuzzlePiece`) (`self.Mesh`))
  (`PrimitiveComponent.SetMaterial` (`self.PuzzlePiece`) 0 (`self.Material`))
  (bind _returnvalue (`GameplayStatics.GetActorOfClass` "/Game/ThirdPerson/Blueprints/BP_FirstPerson.BP_FirstPerson_C"))
  (set `self.PlayerRef` _returnvalue)
  (add `/Game/Alexander/InteractableComponent.OnInteractDispatcher` (`self.InteractableComponent`) (delegate `BeginInteractLogic`)))

(event `BeginInteractLogic`
  (`KismetSystemLibrary.PrintString` "Puzzle interact logic activated")
  (`/Game/ThirdPerson/Blueprints/BP_FirstPerson.InteractStart` (`self.PlayerRef`)))

(fn ` GetPuzzlePiece`
  (returns (Index :type Integer) (PlayerHasPiece :type Boolean) (PieceIsPlaced :type Boolean))
  (return (`self.Index`) true false))

(fn `GetMesh`
  (returns (Name :type Text) (`Static Mesh` :type "StaticMesh Object Reference") (`Item Icon` :type "Texture2D Object Reference"))
  (`/Game/Evert/BP_Painting.SetPuzzlePiece` (`self.Painting`) (`self.Index`) true false)
  (return "Puzzle Piece 1" (`StaticMeshComponent.StaticMesh` (`self.PuzzlePiece`)) (`self.Item Icon`)))

(fn `UserConstructionScript`)
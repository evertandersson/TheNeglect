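; Level loader Blueprint that advances the game through six streamed loop levels.
; Its SwitchLevel event switches on ELevelToLoad, starting a non-blocking unload of that loop and load of the next, visible once loaded.
; The final loop only prints debug text as a placeholder for end-of-game logic.
; Nothing in this graph calls the event or updates the enum.
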(event `self.ReceiveBeginPlay`)

(event `SwitchLevel`
  (switch `/Game/Eryk/LevelLoaders/E_LevelToLoad` (`self.ELevelToLoad`)
    (:`NewEnumerator0`
      (`KismetSystemLibrary.PrintString` "Load level 2")
      (`GameplayStatics.UnloadStreamLevel` "LOOP1")
      (`GameplayStatics.LoadStreamLevel` "LOOP2" true))
    (:`NewEnumerator1`
      (`KismetSystemLibrary.PrintString` "Load level 3")
      (`GameplayStatics.UnloadStreamLevel` "LOOP2")
      (`GameplayStatics.LoadStreamLevel` "LOOP3" true))
    (:`NewEnumerator2`
      (`KismetSystemLibrary.PrintString` "Load level 4")
      (`GameplayStatics.UnloadStreamLevel` "LOOP3")
      (`GameplayStatics.LoadStreamLevel` "LOOP4" true))
    (:`NewEnumerator3`
      (`KismetSystemLibrary.PrintString` "Load level 5")
      (`GameplayStatics.UnloadStreamLevel` "LOOP4")
      (`GameplayStatics.LoadStreamLevel` "LOOP5" true))
    (:`NewEnumerator4`
      (`KismetSystemLibrary.PrintString` "Load level 6")
      (`GameplayStatics.UnloadStreamLevel` "LOOP5")
      (`GameplayStatics.LoadStreamLevel` "LOOP6" true))
    (:`NewEnumerator5`
      (`KismetSystemLibrary.PrintString` "Load level 7")
      (`KismetSystemLibrary.PrintString` "Put end of game logic here"))))

(fn `UserConstructionScript`)